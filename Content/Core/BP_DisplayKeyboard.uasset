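; BP_DisplayKeyboard is a display keyboard that builds its keys at runtime from keyboard data.
; Setup stores the keyboard's details, tags its mesh and the actor for selection by name, then fetches key data by keyboard ID.
; Each key becomes a tagged static mesh component with a material set by keyboard type.
; Regular 40 keys use a fixed rotation without their stored location, while Less Than 40 keys use their full transform.
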(fn `setup`
  (params (keyboardName :type Name) (keyboardType :type "EKeyboard_Type Enum" :default "Regular40") (keyboardStatus :type "EKeyboard_Status Enum" :default "Free") (keyboardStruct :type "KeyboardDataStruct Structure") (keyboardId :type Integer))
  (locals (`static mesh` :type "StaticMesh Soft Object Reference") (NewLocalVar_0 :type "Array of Integer") (NewLocalVar_1 :type "Array of String"))
  (bind _array (`|MakeArray` "keyboard-select" :!type "Name"))
  (bind _componenttags (`ActorComponent.ComponentTags` (`self.KeyboardMesh`)))
  (set `self.keyboardStatus` keyboardStatus)
  (set `self.keyboardType` keyboardType)
  (set `self.keyboardName` keyboardName)
  (bind _output_get (set `self.Keyboard Struct` keyboardStruct))
  (`KismetArrayLibrary.Array_Add` _componenttags "keyboard-select")
  (`KismetArrayLibrary.Array_Add` _componenttags keyboardName)
  (set `self.Tags` _componenttags)
  (bind _newparam (`/Game/Core/functions.Get Keys for Keyboard` (`|MakeArray` keyboardId)))
  (set `self.keycapSpawnDataStructures` _newparam)
  (for _array_element _newparam
    (switch `EKeyboard_Type` (`.keyboardType_12_AFA7D3491A4AE831114D8CA067313D3B` (break `/Game/data/FKeycapSpawnData` _array_element))
      (:`Regular40`
        (bind _returnvalue (`AddComponent|NODE_AddStaticMeshComponent-1` :`RelativeTransform` (`KismetMathLibrary.MakeTransform` (0.0 0.0 0.0) (struct :`Yaw` 90.0) (.scale (`.transform_5_977E05A25048AF0A7B667F961D4D953A` (break `/Game/data/FKeycapSpawnData` _array_element))))))
        (`StaticMeshComponent.SetStaticMesh` _returnvalue (break `/Game/data/FKeycapSpawnData` _array_element))
        (`PrimitiveComponent.SetMaterial` _returnvalue 0 "/Game/Balls/BallMaterial.BallMaterial")
        (set `ActorComponent.ComponentTags` _array _returnvalue))
      (:`LessThan40`
        (bind _returnvalue_2 (`AddComponent|NODE_AddStaticMeshComponent-0` :`RelativeTransform` (`KismetMathLibrary.MakeTransform` (.location (`.transform_5_977E05A25048AF0A7B667F961D4D953A` (break `/Game/data/FKeycapSpawnData` _array_element))) (.rotation (`.transform_5_977E05A25048AF0A7B667F961D4D953A` (break `/Game/data/FKeycapSpawnData` _array_element))) (.scale (`.transform_5_977E05A25048AF0A7B667F961D4D953A` (break `/Game/data/FKeycapSpawnData` _array_element))))))
        (`StaticMeshComponent.SetStaticMesh` _returnvalue_2 (break `/Game/data/FKeycapSpawnData` _array_element))
        (`PrimitiveComponent.SetMaterial` _returnvalue_2 0 "/Game/Environment/Beach/blade.blade")
        (set `ActorComponent.ComponentTags` _array _returnvalue_2)))))

(fn `UserConstructionScript`)