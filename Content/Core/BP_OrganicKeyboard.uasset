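; BP_OrganicKeyboard builds and controls the game's 3D keyboard of BP_Key actors.
; On BeginPlay it spawns child keys, loads organic meshes through the Asset Registry and applies layout labels.
; Functions and events restyle all keys by GetAllActorsOfClass index: cap mesh, left/right colors from the Keys_en table, elevation, spacing, skew and labels.
; Tick animates the Waves elevation, and cap style changes also rotate the directional light.
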(event `self.ReceiveBeginPlay`
  (`self.Generate Organic Keyboard`))

(event `/Game/Core/BPI_Keyboard.setPlayModeKeyStyles`
  (params (val :type String))
  ;[1 1 1] this is in response to the whole game mode changing
  (set `self.playerPlayModeKeyStyle` val))

(event `CustomEvent_6`
  (params (player :type Integer) (val :type String))
  (`|ExecutionSequence`
    (:`then_0`
      (bind _returnvalue (`GameplayStatics.GetActorOfClass` "/Script/Engine.DirectionalLight"))
      (switch `string` val
        (:`tabula`
          (`self.K2_SetActorRotation` _returnvalue (`self.tabula Light Rotation`) false))
        (:`sine`
          (`self.K2_SetActorRotation` _returnvalue (`self.sineLightRotation`) false))
        (:`saw`
          (`self.K2_SetActorRotation` _returnvalue (`self.Saw Light Rotation`) false))
        (:`velum v1`
          (`self.K2_SetActorRotation` _returnvalue (`self.velumLightRotation`) false))))
    (:`then_1`
      (`KismetArrayLibrary.Array_Set` (`self.playerKeyCapTypes`) player val)
      (bind _outactors (`GameplayStatics.GetAllActorsOfClass` "/Game/Core/BP_Key.BP_Key_C"))
      (for (_array_element _array_index) _outactors
        (`self.SwitchKeyCap` val _array_index _array_element)))))

(event `/Game/Core/BPI_Keyboard.BPIsetKeyCapType`
  (params (value :type Name) (index :type Integer) (key :type "/Game/Core/BP_Key Object Reference"))
  (bind _outactors (`GameplayStatics.GetAllActorsOfClass` "/Game/Core/BP_Key.BP_Key_C"))
  (`self.SwitchKeyCap` (`KismetStringLibrary.Conv_NameToString` value) index (`|GetArrayItem` _outactors index)))

(event `/Game/Core/BPI_Keyboard.toggleLabels`
  (set `self.playerLabelsActive` (not (`self.playerLabelsActive`)))
  (bind _outactors (`GameplayStatics.GetAllActorsOfClass` "/Game/Core/BP_Key.BP_Key_C"))
  (for _array_element _outactors
    (set `/Game/Core/BP_Key.labelActive` (`self.playerLabelsActive`) _array_element)))

(event `/Game/Core/BPI_Keyboard.setElevation`
  (params (val :type String))
  (`self.Set Elevation Mode` val))

(event `self.ReceiveTick`
  (params (DeltaSeconds :type "Float (single-precision)"))
  (bind _numberofcolumns (`self.NumberOfColumns`))
  (`|ExecutionSequence`
    (:`then_0`
      (bind _output_get (set `self.tickTimeAccumulation` (+ (`self.tickTimeAccumulation`) DeltaSeconds)))
      (switch `string` (`self.activeElevation`)
        (:`waves`
          (bind _outactors (`GameplayStatics.GetAllActorsOfClass` "/Game/Core/BP_Key.BP_Key_C"))
          (for (_array_element _array_index) _outactors
            (bind _returnvalue (mod (+ (`KismetMathLibrary.FTrunc` _output_get) _array_index) _numberofcolumns))
            ;[1 1 1] wave
            (if (>= _returnvalue (/ _numberofcolumns 2))
              (set `/Game/Core/BP_Key.inactiveZ` (* (`self.stepper val`) (`KismetMathLibrary.Conv_IntToDouble` (- (- (`self.NumberOfColumns`) 1) _returnvalue))) _array_element)
              (else
                (set `/Game/Core/BP_Key.inactiveZ` (* (`self.stepper val`) (`KismetMathLibrary.Conv_IntToDouble` _returnvalue)) _array_element)))))))))

(event `/Game/Core/BPI_Keyboard.setOscillation`
  (set `self.oscillating` true))

(event `/Game/Core/BPI_Keyboard.Space Bump`
  (params (rumble :type Boolean))
  (bind _outactors (`GameplayStatics.GetAllActorsOfClass` "/Game/Core/BP_Key.BP_Key_C"))
  (for _array_element _outactors
    (set `/Game/Core/BP_Key.isActive` rumble _array_element)))

(event `/Game/Core/BPI_Keyboard.set Symbol Layout`
  (params (player :type Integer) (val :type String))
  (`KismetSystemLibrary.PrintString` val)
  (`self.updateLayout` val))

(fn `Assign Relative Positions`
  (params (Key :type "/Game/Core/BP_Key Object Reference") (index :type Integer))
  (locals (alphacount :type Integer))
  (bind _key (`self.Key`))
  (bind _col (`/Game/Core/BP_Key.col` Key))
  (set `local.alphacount` index)
  ;[1 1 1] detect position ( side, corner, center )
  (set `self.Key` Key)
  (if (and (== _col 0) (== (`local.alphacount`) 0))
    (set `/Game/Core/BP_Key.relativePosition` "topleft" _key)
    (elif (== index (- (`KismetArrayLibrary.Array_Length` (`self.alphabetArray`)) (`self.rowLength`)))
      (set `/Game/Core/BP_Key.relativePosition` "bottomleft" _key)
      (elif (== _col 0)
        (set `/Game/Core/BP_Key.relativePosition` "left" _key)
        (elif (== (`local.alphacount`) (- (`KismetArrayLibrary.Array_Length` (`self.alphabetArray`)) 1))
          (set `/Game/Core/BP_Key.relativePosition` "bottomright" _key)
          (elif (> (`local.alphacount`) (- (`KismetArrayLibrary.Array_Length` (`self.alphabetArray`)) (`self.rowLength`)))
            (set `/Game/Core/BP_Key.relativePosition` "bottom" _key)
            (elif (== (`local.alphacount`) (- (`self.rowLength`) 1))
              (set `/Game/Core/BP_Key.relativePosition` "topright" _key)
              (elif (== (- (`self.rowLength`) 1) _col)
                (set `/Game/Core/BP_Key.relativePosition` "right" _key)
                (elif (< (`local.alphacount`) (`self.rowLength`))
                  (set `/Game/Core/BP_Key.relativePosition` "top" _key)
                  (else
                    (set `/Game/Core/BP_Key.relativePosition` "center" _key)))))))))))

(fn `continueKeyboardCustomisation`
  (params (index :type Integer) (newKeyValue :type String))
  (locals (col :type "LinearColor Structure") (ActivelyCustomisingKeyIndex :type Integer))
  ;[1 1 1] set temporary label in key at index, highlight next key
)

(fn `Generate Organic Keyboard`
  (locals (KeyColor :type "Color Structure") (keyEmitter :type "Color Structure") (NewLocalVar_4 :type "AssetData Structure"))
  (bind _returnvalue (`AssetRegistryHelpers.GetAssetRegistry`))
  ;[1 1 1] remove existing keys if they exist??? does this cause bugs??
  (for _array_element (`self.GetAllChildActors` true)
    (`self.K2_DestroyActor` _array_element))
  (for _ (range (* (`self.NumberOfRows`) (`self.NumberOfColumns`)))
    (`AddComponent|NODE_AddChildActorComponent-6` :`bManualAttachment` true))
  ;[1 1 1] load and assign organic meshes
  (bind _outactors (`GameplayStatics.GetAllActorsOfClass` "/Game/Core/BP_Key.BP_Key_C"))
  (set `self.keys` _outactors)
  (bind _outassetdata (message `AssetRegistry.GetAssetsByPath` (`KismetSystemLibrary.Conv_InterfaceToObject` _returnvalue) "/Game/Keys/weird/weird1" false false))
  (`KismetSystemLibrary.PrintString` (`KismetStringLibrary.Conv_IntToString` (`KismetArrayLibrary.Array_Length` _outassetdata)))
  (message `AssetRegistry.RunAssetsThroughFilter` (`KismetSystemLibrary.Conv_InterfaceToObject` _returnvalue) _outassetdata (make `ARFilter` :`ClassNames` (`self.NewLocalVar_3`)))
  (for (_array_element_2 _array_index) _outassetdata
    (bind _output_get (set `local.NewLocalVar_4` _array_element_2))
    (bind _returnvalue_2 (`KismetStringLibrary.Conv_NameToString` (`.AssetName` (break `AssetData` _output_get))))
    (`KismetSystemLibrary.PrintString` (`KismetStringLibrary.Concat_StrStr` (`KismetStringLibrary.Conv_IntToString` _array_index) "  " _returnvalue_2))
    (bind _output (`|GetArrayItem` _outactors _array_index))
    (set `/Game/Core/BP_Key.organic_index` (`KismetStringLibrary.Conv_StringToInt` _returnvalue_2) _output)
    (set `Actor.Tags` (`|MakeArray` (`KismetStringLibrary.Conv_StringToName` _returnvalue_2)) _output)
    (bind _asstatic_mesh (cast `StaticMesh` (`AssetRegistryHelpers.GetAsset` _array_element_2))
      (:`then`
        (`/Game/Core/BP_Key.setOrganicKeyMesh` _output _asstatic_mesh))
      (:`CastFailed`
        (`KismetSystemLibrary.PrintString` "couldnt turn something into static mesh"))))
  ;[1 1 1] add labels
  (`self.updateLayout` (`self.Selected Keyboard Layout`) true))

(fn `getColorsAndEmitters`
  (params (capType :type String))
  (returns (color1 :type "Color Structure") (emitter1 :type "Color Structure") (color2 :type "Color Structure") (emitter2 :type "Color Structure"))
  (for _array_element (`self.key details and colors`)
    (if (`KismetTextLibrary.EqualEqual_TextText` (break `/Game/data/KeyDetails` _array_element) (`KismetTextLibrary.Conv_StringToText` capType))
      (return (`.color1_29_DE125A564B16CB0604820A9DD16C06F2` (break `/Game/data/KeyDetails` _array_element)) (`.emitter1_26_E37321DA4F51130E3FE328A71F5FCB7E` (break `/Game/data/KeyDetails` _array_element)) (`.color2_27_BE22179B427530F503665C89478E4D07` (break `/Game/data/KeyDetails` _array_element)) (`.emitter2_28_C203ED3D457E3068C36639BEE8F68B75` (break `/Game/data/KeyDetails` _array_element))))))

(fn `oscillate`
  (if (`self.oscillating`)
    (bind _output_get (set `self.flipped` (not (`self.flipped`))))
    (if _output_get
      (`self.setKeySpacing` "medium")
      (else
        (`self.setKeySpacing` "big")))))

(fn `Set Elevation Mode`
  (params (val :type String))
  (bind _returnvalue (`GameplayStatics.GetGameState`))
  (bind _numberofcolumns (`self.NumberOfColumns`))
  (bind _numberofcolumns_2 (`self.NumberOfColumns`))
  (bind _elevationloopindex (`self.ElevationLoopIndex`))
  (bind _elevationkey (`self.ElevationKey`))
  (bind _numberofcolumns_3 (`self.NumberOfColumns`))
  (bind _returnvalue_2 (* (`self.NumberOfColumns`) (`self.stepper val`)))
  (bind _returnvalue_3 (mod (`self.ElevationLoopIndex`) _numberofcolumns_3))
  (bind _returnvalue_4 (mod (`self.ElevationLoopIndex`) _numberofcolumns))
  (`|ExecutionSequence`
    (:`then_0`
      (set `self.activeElevation` val)
      (bind _outactors (`GameplayStatics.GetAllActorsOfClass` "/Game/Core/BP_Key.BP_Key_C"))
      (for (_array_element _array_index) _outactors
        (set `self.ElevationKey` _array_element)
        (set `self.ElevationLoopIndex` _array_index)
        (switch `string` (`self.activeElevation`)
          (:`flat`
            ;[1 1 1] flat
            (set `/Game/Core/BP_Key.inactiveZ` 0.0 (`self.ElevationKey`)))
          (:`valley`
            ;[1 1 1] valley
            (if (>= _returnvalue_4 (/ _numberofcolumns 2))
              (set `/Game/Core/BP_Key.inactiveZ` (- (* (`self.stepper val`) (`KismetMathLibrary.Conv_IntToDouble` (- _numberofcolumns_2 (- (- _numberofcolumns_2 1) _returnvalue_4)))) _returnvalue_2) (`self.ElevationKey`))
              (else
                (set `/Game/Core/BP_Key.inactiveZ` (- (* (`self.stepper val`) (`KismetMathLibrary.Conv_IntToDouble` (- _numberofcolumns_2 _returnvalue_4))) _returnvalue_2) (`self.ElevationKey`)))))
          (:`stairs center`
            ;[1 1 1] stairs center
            (if (>= _returnvalue_3 (/ _numberofcolumns_3 2))
              (set `/Game/Core/BP_Key.inactiveZ` (* (`self.stepper val`) (`KismetMathLibrary.Conv_IntToDouble` (- (- (`self.NumberOfColumns`) 1) _returnvalue_3))) (`self.ElevationKey`))
              (else
                (set `/Game/Core/BP_Key.inactiveZ` (* (`self.stepper val`) (`KismetMathLibrary.Conv_IntToDouble` _returnvalue_3)) (`self.ElevationKey`)))))
          (:`stairs right`
            ;[1 1 1] stairs right
            (set `/Game/Core/BP_Key.inactiveZ` (* (`KismetMathLibrary.Conv_IntToDouble` (mod _elevationloopindex (`self.NumberOfColumns`))) (`self.stepper val`)) (`self.ElevationKey`)))
          (:`stairs left`
            ;[1 1 1] stairs left
            (set `/Game/Core/BP_Key.inactiveZ` (* (`KismetMathLibrary.Conv_IntToDouble` (- (`self.NumberOfColumns`) (mod _elevationloopindex (`self.NumberOfColumns`)))) (`self.stepper val`)) (`self.ElevationKey`)))
          (:`bench`
            ;[1 1 1] bench
            (set `/Game/Core/BP_Key.inactiveZ` (`KismetMathLibrary.Conv_IntToDouble` (* (`/Game/Core/BP_Key.row` _elevationkey) -10)) _elevationkey)))))
    (:`then_1`
      (bind _playmode (message `/Game/Core/BPI_GameState.getPlayMode` _returnvalue))
      (if (not (`KismetStringLibrary.EqualEqual_StrStr` _playmode "keyball"))
        (message `/Game/Core/BPI_GameState.setPlayMode` _returnvalue "keyball")))))

(fn `Set Key Skewing`
  (params (Val :type String))
  (locals (offset :type "Float (double-precision)"))
  (switch `string` Val
    (:`uniform`
      (set `local.offset` 0.0))
    (:`skewed`
      (set `local.offset` 10.0)))
  (bind _outactors (`GameplayStatics.GetAllActorsOfClass` "/Game/Core/BP_Key.BP_Key_C"))
  (for _array_element _outactors
    (set `/Game/Core/BP_Key.targetSkewOffset` (`local.offset`) _array_element)))

(fn `setKeySpacing`
  (params (val :type String))
  (bind _outactors (`GameplayStatics.GetAllActorsOfClass` "/Game/Core/BP_Key.BP_Key_C"))
  (for (_array_element _array_index) _outactors
    (switch `string` val
      (:`closed`
        (set `/Game/Core/BP_Key.targetPosition` (`|GetArrayItem` (`self.margins_closed`) _array_index) _array_element))
      (:`medium`
        (set `/Game/Core/BP_Key.targetPosition` (`|GetArrayItem` (`self.margins_medium`) _array_index) _array_element))
      (:`big`
        (set `/Game/Core/BP_Key.targetPosition` (`|GetArrayItem` (`self.margins_big`) _array_index) _array_element))
      (:`oscillate`
        (set `self.oscillating` true)))))

(fn `String to Array`
  (params (alphabetString :type String))
  (returns (alphabetArray :type "Array of String"))
  (return (`KismetStringLibrary.ParseIntoArray` alphabetString " " false)))

(fn `SwitchKeyCap`
  (params (Selection :type String) (KeyPositionIndex :type Integer) (KeyCapArrayElement :type "/Game/Core/BP_Key Object Reference"))
  (locals (NewLocalVar_0 :type "Color Structure") (keyColor :type "Color Structure") (keyEmitter :type "Color Structure"))
  (bind _keycaparrayelement (`self.KeyCapArrayElement`))
  (bind _numberofcolumns (`self.NumberOfColumns`))
  (bind _keycaparrayelement_2 (`self.KeyCapArrayElement`))
  (bind _rowlength (`self.rowLength`))
  (bind _returnvalue (`KismetMathLibrary.Conv_ColorToLinearColor` (`local.keyColor`)))
  (bind _returnvalue_2 (`KismetMathLibrary.Conv_ColorToLinearColor` (`local.keyEmitter`)))
  (bind _returnvalue_3 (`KismetMathLibrary.Conv_ColorToLinearColor` (`local.keyColor`)))
  (bind _returnvalue_4 (`KismetMathLibrary.Conv_ColorToLinearColor` (`local.keyEmitter`)))
  (set `self.Selection` Selection)
  (set `self.KeyCapArrayElement` KeyCapArrayElement)
  (set `self.KeyCapArrayIndex` KeyPositionIndex)
  (bind (_color1 _emitter1 _color2 _emitter2) (`self.getColorsAndEmitters` (`self.Selection`)))
  (if (> (mod KeyPositionIndex _rowlength) (/ _rowlength 2))
    ;[1 1 1] right side colors
    (set `local.keyColor` _color2)
    (set `local.keyEmitter` _emitter2)
    (else
      ;[1 1 1] left side colors
      (set `local.keyColor` _color1)
      (set `local.keyEmitter` _emitter1)))
  (switch `string` (`self.Selection`)
    (:`Default`
      (`/Game/Core/BP_Key.Set Key Mesh` _keycaparrayelement_2 (`KismetStringLibrary.Conv_StringToName` (`self.Selection`)) (`KismetMathLibrary.Conv_ColorToLinearColor` (`local.keyColor`)) (`KismetMathLibrary.Conv_ColorToLinearColor` (`local.keyEmitter`)) false))
    (:`saw`
      ;[1 1 1] saw cap
      (if (< (mod (`self.KeyCapArrayIndex`) _numberofcolumns) (/ _numberofcolumns 2))
        (`/Game/Core/BP_Key.Set Key Mesh` _keycaparrayelement "sawleft" _returnvalue _returnvalue_2 false)
        (else
          (`/Game/Core/BP_Key.Set Key Mesh` _keycaparrayelement "sawright" _returnvalue _returnvalue_2 false))))
    (:`sine`
      ;[1 1 1] SINE CAP
      (if (== (mod (`self.KeyCapArrayIndex`) 2) 0)
        (`/Game/Core/BP_Key.Set Key Mesh` _keycaparrayelement_2 "sine1" _returnvalue_3 _returnvalue_4 false)
        (else
          (`/Game/Core/BP_Key.Set Key Mesh` _keycaparrayelement_2 "sine2" _returnvalue_3 _returnvalue_4 false))))
    (:`tabula`
      (`/Game/Core/BP_Key.Set Key Mesh` _keycaparrayelement_2 "tabula" (`KismetMathLibrary.Conv_ColorToLinearColor` (`local.keyColor`)) (`KismetMathLibrary.Conv_ColorToLinearColor` (`local.keyEmitter`)) false))
    (:`velum v1`
      (`/Game/Core/BP_Key.Set Key Mesh` _keycaparrayelement_2 "velumv1" (`KismetMathLibrary.Conv_ColorToLinearColor` (`local.keyColor`)) (`KismetMathLibrary.Conv_ColorToLinearColor` (`local.keyEmitter`)) false))))

(fn `updateLayout`
  (params (layout :type String) (organic :type Boolean))
  (locals (local_keys :type "Array of /Game/Core/BP_Key Object Reference"))
  (bind _value (`BlueprintMapLibrary.Map_Find` (`self.KeyboardLayouts`) layout))
  ;[1 1 1] layout refers to keyboard key labels, not position or orientation etc.
  (bind _outactors (`GameplayStatics.GetAllActorsOfClass` "/Game/Core/BP_Key.BP_Key_C"))
  (set `local.local_keys` _outactors)
  (bind _alphabetarray (`self.String to Array` _value))
  (`KismetSystemLibrary.PrintString` _value)
  (bind _output_get (set `self.alphabetArray` _alphabetarray))
  (if organic
    (for (_ _array_index) _output_get
      (for _array_element (`local.local_keys`)
        (if (`self.ActorHasTag` _array_element (`KismetStringLibrary.Conv_StringToName` (`KismetStringLibrary.Concat_StrStr` "m" (`KismetStringLibrary.Conv_IntToString` _array_index))))
          (bind _output (`|GetArrayItem` (`self.alphabetArray`) _array_index))
          (bind (_value_2 _returnvalue) (`BlueprintMapLibrary.Map_Find` (`self.odd_strings`) _output))
          ;[1 1 1] set name (not always same as symbol?)
          (if _returnvalue
            (set `/Game/Core/BP_Key.name` _value_2 _array_element)
            (else
              (set `/Game/Core/BP_Key.name` _output _array_element)))
          ;[1 1 1] eg. a,b,c,5,3,.
          (set `/Game/Core/BP_Key.symbol` _output _array_element))))
    (else
      (bind (_arrayindex _arrayelement) (`/Engine/EditorBlueprintResources/StandardMacros.ReverseForEachLoop` (`local.local_keys`))
        (:`LoopBody`
          (bind _output_2 (`|GetArrayItem` (`self.alphabetArray`) _arrayindex))
          (bind (_value_3 _returnvalue_2) (`BlueprintMapLibrary.Map_Find` (`self.odd_strings`) _output_2))
          ;[1 1 1] set name (not always same as symbol?)
          (if _returnvalue_2
            (set `/Game/Core/BP_Key.name` _value_3 _arrayelement)
            (else
              (set `/Game/Core/BP_Key.name` _output_2 _arrayelement)))
          ;[1 1 1] eg. a,b,c,5,3,.
          (set `/Game/Core/BP_Key.symbol` _output_2 _arrayelement))))))

(fn `UserConstructionScript`
  (locals (NewLocalVar_1 :type "AssetData Structure") (NewLocalVar_2 :type "Array of Name"))
  (bind _outrownames (`DataTableFunctionLibrary.GetDataTableRowNames` "/Game/data/keys_en.keys_en"))
  (for _array_element _outrownames
    (bind _returnvalue (`|GetDataTableRow` "/Game/data/keys_en.keys_en" _array_element)
      (:`then`
        (`KismetArrayLibrary.Array_Add` (`self.key details and colors`) _returnvalue))))
  (bind _returnvalue_2 (`GameplayStatics.LoadGameFromSlot` "keyball"))
  (bind _asbp_save_game (cast `/Game/Core/BP_SaveGame` _returnvalue_2)
    (:`CastFailed`
      (`KismetSystemLibrary.PrintString` "failed to load game, please tell us in discord"))))

(fn `whichPlayer`
  (params (index :type Integer))
  (returns (playerIndex :type Integer))
  (bind _rowlength (`self.rowLength`))
  (if (>= (mod index _rowlength) (/ _rowlength 2))
    (return 1)
    (else
      (return 0))))