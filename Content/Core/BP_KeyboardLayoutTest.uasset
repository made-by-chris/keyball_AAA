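; BP_KeyboardLayoutTest is a debug actor for testing keyboard-layout-aware key mapping.
; Pressing Z converts the key's code through MapKeyToQWERTY and prints the resulting QWERTY key name joined with the original key's display name, after a "Hello" message.
; An unconnected branch would print the current keyboard layout after a delay, but it never runs.
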(event `self.ReceiveBeginPlay`)

(event `Key|Z`
  (params (Key :type "Key Structure"))
  (:`Pressed`
    (`KismetSystemLibrary.PrintString` "Hello")
    (bind _returnvalue (`KeyboardLayoutDetector.MapKeyToQWERTY` (`Keyball_Function_Library.GetKeyCode` Key)))
    (`KismetSystemLibrary.PrintString` (`KismetStringLibrary.Concat_StrStr` (`KismetTextLibrary.Conv_TextToString` (`KismetInputLibrary.Key_GetDisplayName` _returnvalue)) (`KismetTextLibrary.Conv_TextToString` (`KismetInputLibrary.Key_GetDisplayName` Key))))))

(fn `UserConstructionScript`)