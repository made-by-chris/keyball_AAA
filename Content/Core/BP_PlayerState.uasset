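; Player state that holds each player's team number and preferred keyboard layout.
; On BeginPlay, only when the game instance flags a fresh start, it copies the saved layout into the preferred, primary and secondary fields, then clears the flag.
; Setting a new preferred layout also updates the first BP_Keyboard actor found.
; The layout's RepNotify handler is empty.
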(event `set player initial values computed from server`
  (params (NewParam :type Boolean) (TeamNumber :type Integer))
  (set `self.TeamNumber` TeamNumber))

(event `/Game/Core/BPI_PlayerState.setPreferedLayout`
  (params (`layout or language` :type String))
  (bind _output_get (set `self.preferedLayout` `layout or language`))
  (bind _returnvalue (`GameplayStatics.GetActorOfClass` "/Game/Core/BP_Keyboard.BP_Keyboard_C"))
  (`/Game/Core/BP_Keyboard.Update Layout` _returnvalue _output_get))

(event `self.ReceiveBeginPlay`
  ;[1 1 1] if game is just starting AKA we're not just switching levels or something
  (bind _asbp_game_instance (cast `/Game/Core/BP_GameInstance` (`GameplayStatics.GetGameInstance`)))
  (if (`/Game/Core/BP_GameInstance.game is just starting` _asbp_game_instance)
    (bind _asbp_game_instance_2 (cast `/Game/Core/BP_GameInstance` (`GameplayStatics.GetGameInstance`)))
    (bind _keyboardlayout (`/Game/Core/BP_GameInstance.KeyboardLayout` _asbp_game_instance_2))
    ;[1 1 1] can be used in multiplayer to determine which layouts etc to show
    (set `self.preferedLayout` _keyboardlayout)
    (set `self.preferedPrimary` (`KismetStringLibrary.Conv_StringToName` _keyboardlayout))
    (set `self.preferedSecondary` (`KismetStringLibrary.Conv_StringToName` _keyboardlayout))
    (set `/Game/Core/BP_GameInstance.game is just starting` false _asbp_game_instance)))

(fn `get player state`
  (returns (`player state ` :type "/Game/Core/BP_PlayerState Object Reference"))
  (return self))

(fn `OnRep_preferedLayout`)

(fn `UserConstructionScript`)