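; Game camera actor that switches behaviour by CamMode, with the starting mode chosen from the level name.
; Dynamic mode damps the ball's movement and pitches toward the keyboard-ball midpoint, while Spin modes orbit the keyboard facing the ball.
; Home Screen leans its aim slightly toward the cursor, and other modes ease to preset poses.
; Each tick also eases the camera component sideways for the Home Screen's 2D menu.
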(event `self.ReceiveTick`
  (params (DeltaSeconds :type "Float (single-precision)"))
  (bind _returnvalue (`self.K2_GetActorLocation`))
  (bind _cameracomponent (`self.CameraComponent`))
  (bind (_relativelocation_x _relativelocation_y _relativelocation_z) (`KismetMathLibrary.BreakVector` (`SceneComponent.RelativeLocation` _cameracomponent)))
  (bind (_returnvalue_x _returnvalue_y _returnvalue_z) (`KismetMathLibrary.BreakVector` (`SceneComponent.K2_GetComponentLocation` (`/Game/Core/BP_PhysicsObject.Sphere` (`self.ball`)))))
  (bind (_returnvalue_x_2 _returnvalue_y_2 _returnvalue_z_2) (`KismetMathLibrary.BreakVector` (`SceneComponent.K2_GetComponentLocation` (`Actor.RootComponent` (`self.ball`)))))
  (bind (_returnvalue_x_3 _returnvalue_y_3 _returnvalue_z_3) (`KismetMathLibrary.BreakVector` (/ (+ (`self.K2_GetActorLocation` (`self.keyboard`)) (`self.K2_GetActorLocation` (`self.ball`))) 2.0)))
  (set `self.Delta Seconds` DeltaSeconds)
  (`|ExecutionSequence`
    (:`then_0`
      (if (not (`KismetSystemLibrary.IsValid` (`self.ball`)))
        (bind _returnvalue_2 (`GameplayStatics.GetActorOfClass` "/Game/Core/BP_PhysicsObject.BP_PhysicsObject_C"))
        (set `self.ball` _returnvalue_2))
      (switch `string` (`self.camMode`)
        (:`dynamic`
          (`/Game/Core/functions.Tick Lerp Location` self (`KismetMathLibrary.MakeVector` -340.0 (/ _returnvalue_y 2.0) (+ (`self.camHeight`) (/ (- _returnvalue_z 200.0) 5.0))) (`self.Delta Seconds`))
          (`/Game/Core/functions.Tick Lerp Rotation` self (`KismetMathLibrary.FindLookAtRotation` _returnvalue (`KismetMathLibrary.MakeVector` _returnvalue_x_3 (.y _returnvalue) _returnvalue_z_3)) (/ (`self.Delta Seconds`) 3.0)))
        (:`customise layout`
          (`/Game/Core/functions.Tick Lerp To` self (`self.custom layout cam rotation`) (`self.custom layout cam location`) DeltaSeconds))
        (:`spin`
          (set `self.spreed` 3.0)
          (bind _output_get (set `self.spin direction` (- (`self.K2_GetActorLocation`) (`SceneComponent.K2_GetComponentLocation` (`Actor.RootComponent` (`self.keyboard`)))) :!label _label))
          (`SceneComponent.K2_AddWorldOffset` (`self.SceneComponent`) (- (`KismetMathLibrary.RotateAngleAxis` _output_get (* (`self.spreed`) (`GameplayStatics.GetWorldDeltaSeconds`)) (0.0 0.0 1.0)) (`self.spin direction`)) true false)
          (`SceneComponent.K2_SetWorldRotation` (`self.SceneComponent`) (`KismetMathLibrary.FindLookAtRotation` (`SceneComponent.K2_GetComponentLocation` (`self.SceneComponent`)) (`KismetMathLibrary.MakeVector` _returnvalue_x_2 _returnvalue_y_2 _returnvalue_z_2)) false false))
        (:`spin reverse`
          (set `self.spreed` -3.0)
          (goto _label))
        (:`HomeScreen`
          (`/Game/Core/functions.Tick Lerp To` self (`KismetMathLibrary.FindLookAtRotation` (`SceneComponent.K2_GetComponentLocation` (`self.CameraComponent`)) (`KismetMathLibrary.VLerp` (`self.center looky point`) (`.Location` (`GameplayStatics.BreakHitResult` (`PlayerController.GetHitResultUnderCursorByChannel` (`GameplayStatics.GetPlayerController` 0) "TraceTypeQuery1" true))) 0.1)) (`self.HomeScreen Cam Location`) DeltaSeconds))
        (:`computer`
          (`/Game/Core/functions.Tick Lerp To` self (struct :`Yaw` 2.0) (`self.phone out camera position`) DeltaSeconds))
        (:`boot zoom`
          (`/Game/Core/functions.Tick Lerp To` self (`self.boot rotation`) (`self.boot location`) DeltaSeconds))))
    (:`then_1`
      (`SceneComponent.K2_SetRelativeLocation` _cameracomponent (`KismetMathLibrary.MakeVector` _relativelocation_x (`KismetMathLibrary.Lerp` _relativelocation_y (select `bool` (and (`self.2d menu active`) (`KismetStringLibrary.EqualEqual_StrStr` (`self.camMode`) "HomeScreen")) :`true` (`self.2d menu active offset`)) (* DeltaSeconds 3.0)) _relativelocation_z) false false))))

(event `self.ReceiveBeginPlay`
  (bind _returnvalue (`GameplayStatics.GetActorOfClass` "/Game/Core/BP_Keyboard.BP_Keyboard_C"))
  (set `self.keyboard` _returnvalue)
  (set `self.Computer Camera Location` null)
  (bind _returnvalue_2 (`GameplayStatics.GetCurrentLevelName` true))
  (switch `string` _returnvalue_2
    (:`Default`
      (set `self.camMode` "dynamic" :!label _label_2))
    (:`HomeScreen`
      (set `self.camMode` "HomeScreen"))
    (:`Multiplayer`
      (goto _label_2))))

(fn `UserConstructionScript`
  (bind (_returnvalue_x _returnvalue_y _returnvalue_z) (`KismetMathLibrary.BreakVector` (`self.K2_GetActorLocation`)))
  (set `self.HomeScreen Cam Location` (`KismetMathLibrary.MakeVector` (+ _returnvalue_x 100.0) _returnvalue_y _returnvalue_z))
  (set `self.HomeScreen Cam Rotation` (`self.K2_GetActorRotation`)))