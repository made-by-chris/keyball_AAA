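; Replicated keyboard key actor with swappable keycap or organic meshes, a widget label and a state-colored LED outline.
; SetKeyActive sets press height, speed and LED state from shift, double-tap and cooldown.
; On authority, Tick interpolates actor position, inner key travel, row skew and tilt.
; OnRep functions refresh materials, outline and cooldown timer, while a toggle picks each team's primary or secondary keycap from the active mod message.
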(event `update outline`
  (switch `string` (`self.LED State`)
    (:`active`
      (set `self.outline color` (make `Color` 255 255 255 1)))
    (:`fast active`
      (set `self.outline color` (make `Color` 0 255 0 1)))
    (:`inactive`
      (set `self.outline color` (make `Color` 100 100 100)))
    (:`shift active`
      (set `self.outline color` (make `Color` 255 215 0 1)))
    (:`cooldown`
      (set `self.outline color` (make `Color` 0 100 255 1))))
  (bind _returnvalue (`PrimitiveComponent.CreateDynamicMaterialInstance` (`self.StaticMeshForOutline`) 0 "/Game/Materials/M_Outline.M_Outline" "None"))
  (`MaterialInstanceDynamic.SetVectorParameterValue` _returnvalue "Color" (`KismetMathLibrary.Conv_ColorToLinearColor` (`self.outline color`)))
  (`MaterialInstanceDynamic.SetVectorParameterValue` _returnvalue "Emitter" (`KismetMathLibrary.Conv_ColorToLinearColor` (`self.outline color`)))
  (`MaterialInstanceDynamic.SetScalarParameterValue` _returnvalue "Opacity" (select `bool` (`KismetStringLibrary.EqualEqual_StrStr` (`self.LED State`) "inactive") :`false` 1.0 :!type "Float (single-precision)")))

(event `self.ReceiveBeginPlay`
  (bind _returnvalue (`KismetSystemLibrary.GetGameTimeInSeconds`))
  (set `self.Last Pressed` _returnvalue)
  (set `self.Last Released` (- _returnvalue 100.0))
  (`LightComponent.SetLightColor` (`self.RectLight`) (`KismetMathLibrary.Conv_ColorToLinearColor` (`self.LED Colour`)) true)
  (bind _asw_key_label (cast `/Game/Core/W_KeyLabel` (`WidgetComponent.GetWidget` (`self.LabelTarget`))))
  (set `/Game/Core/W_KeyLabel.LED COLOR` (make `SlateColor` (struct :`R` 1.0 :`B` 1.0 :`A` 1.0)) _asw_key_label))

(event `self.ReceiveTick`
  (params (DeltaSeconds :type "Float (single-precision)"))
  (bind (_returnvalue_x _returnvalue_y _returnvalue_z) (`KismetMathLibrary.BreakVector` (`self.K2_GetActorLocation`)))
  (bind (_returnvalue_x_2 _returnvalue_y_2 _returnvalue_z_2) (`KismetMathLibrary.BreakVector` (`self.K2_GetActorLocation`)))
  (bind (_returnvalue_x_3 _returnvalue_y_3) (`KismetMathLibrary.BreakVector` (`self.K2_GetActorLocation`)))
  (bind _staticmesh (`self.StaticMesh`))
  (bind _final_z_active_value_after_behavior_check (`self.final Z Active Value After Behavior Check`))
  (bind _staticmesh_2 (`self.StaticMesh`))
  (bind _staticmesh_3 (`self.StaticMesh`))
  (bind (_returnvalue_x_4 _returnvalue_y_4) (`KismetMathLibrary.BreakVector` (`KismetMathLibrary.VLerp` (`self.K2_GetActorLocation`) (`self.targetPosition`) 0.1)))
  (bind (_relativelocation_x _relativelocation_y _relativelocation_z) (`KismetMathLibrary.BreakVector` (`SceneComponent.RelativeLocation` _staticmesh_3)))
  (bind (_relativelocation_x_2 _relativelocation_y_2 _relativelocation_z_2) (`KismetMathLibrary.BreakVector` (`SceneComponent.RelativeLocation` _staticmesh_2)))
  (bind _returnvalue (`KismetMathLibrary.Lerp` _relativelocation_y (* (`self.row_multiplyer`) (`self.targetSkewOffset`)) 0.1))
  (set `self.Delta Seconds` DeltaSeconds)
  (`SceneComponent.SetVisibility` (`self.LabelTarget`) (`self.labelActive`) false)
  (`/Engine/EditorBlueprintResources/ActorMacros.Switch Has Authority`
    (:`Authority`
      (`|ExecutionSequence`
        (:`then_0`
          (switch `name` (`self.KeyCapType`)
            (:`trickyv1`
              (`SceneComponent.K2_AddLocalRotation` (`self.StaticMesh`) (struct :`Yaw` 1.0) false false))))
        (:`then_1`
          ;[1 1 1] Outer Key height ( for stepping, waves )
          (if true
            (`self.K2_SetActorLocation` (`KismetMathLibrary.MakeVector` _returnvalue_x_3 _returnvalue_y_3 (`KismetMathLibrary.FInterpTo` _returnvalue_z (`self.inactiveZ`) DeltaSeconds 2.0)))))
        (:`then_2`
          ;[1 1 1] Inner (relative) Key height (for user controls)
          (if (and (`self.isActive`) (not (and (`self.Tilt Is Active`) (`self.Shift Is Active`))))
            (if (> (`KismetSystemLibrary.GetGameTimeInSeconds`) (+ (`self.Last Released`) (`self.cooldown`)))
              (set `self.final Z Active Value After Behavior Check` (`self.Z_Active_Value`))
              (if (not (== _final_z_active_value_after_behavior_check _relativelocation_z_2))
                (`SceneComponent.K2_SetRelativeLocation` _staticmesh_2 (`KismetMathLibrary.MakeVector` _relativelocation_x_2 _relativelocation_y_2 (`KismetMathLibrary.Lerp` _relativelocation_z_2 _final_z_active_value_after_behavior_check (`self.key speed`))) false false)))
            (elif (not (== _relativelocation_z_2 0.0))
              (`SceneComponent.K2_SetRelativeLocation` _staticmesh_2 (`KismetMathLibrary.MakeVector` _relativelocation_x_2 _relativelocation_y_2 (`KismetMathLibrary.Lerp` _relativelocation_z_2 0.0 (`self.key speed`))) false false))))
        (:`then_3`
          ;[1 1 1] if this is too slow (0.005) it fucks with collision
          (`self.K2_SetActorLocation` (`KismetMathLibrary.MakeVector` _returnvalue_x_4 _returnvalue_y_4 _returnvalue_z_2) true))
        (:`then_4`
          ;[1 1 1] JPEG / PNG ( RE-ADD ME )
          (`SceneComponent.K2_SetRelativeLocation` (`self.LabelTarget`) (`KismetMathLibrary.MakeVector` _relativelocation_x _returnvalue (+ _relativelocation_z 10.0)) false false)
          (switch `int` (`self.row`)
            (:`0`
              (set `self.row_multiplyer` -2))
            (:`1`
              (set `self.row_multiplyer` -1))
            (:`2`
              (set `self.row_multiplyer` 1))
            (:`3`
              (set `self.row_multiplyer` 2)))
          (`SceneComponent.K2_SetRelativeLocation` _staticmesh_3 (`KismetMathLibrary.MakeVector` _relativelocation_x _returnvalue _relativelocation_z) false false))
        (:`then_5`
          ;[1 1 1] rotate keys ( if tilt rotation is changed due to tilting or other stuff )
          (`SceneComponent.K2_SetRelativeRotation` _staticmesh (`KismetMathLibrary.Conv_VectorToRotator` (`KismetMathLibrary.VLerp` (`KismetMathLibrary.Conv_RotatorToVector` (`SceneComponent.RelativeRotation` _staticmesh)) (`KismetMathLibrary.Conv_RotatorToVector` (`self.Tilt Rotation`)) (* DeltaSeconds 10.0))) false false))))))

(fn `cooldown ended`
  (set `self.LED State` "inactive"))

(fn `OnRep_color`
  (bind _returnvalue (`PrimitiveComponent.CreateDynamicMaterialInstance` (`self.StaticMesh`) 0 "/Game/Keys/KeyMaterial.KeyMaterial" "None"))
  (`MaterialInstanceDynamic.SetVectorParameterValue` _returnvalue "Color" (`KismetMathLibrary.Conv_ColorToLinearColor` (`self.color`)))
  (`MaterialInstanceDynamic.SetVectorParameterValue` _returnvalue "Emitter" (`KismetMathLibrary.Conv_ColorToLinearColor` (`self.emitter`))))

(fn `OnRep_emitter`
  (bind _returnvalue (`PrimitiveComponent.CreateDynamicMaterialInstance` (`self.StaticMesh`) 0 "/Game/Keys/KeyMaterial.KeyMaterial" "None"))
  (`MaterialInstanceDynamic.SetVectorParameterValue` _returnvalue "Color" (`KismetMathLibrary.Conv_ColorToLinearColor` (`self.color`)))
  (`MaterialInstanceDynamic.SetVectorParameterValue` _returnvalue "Emitter" (`KismetMathLibrary.Conv_ColorToLinearColor` (`self.emitter`))))

(fn `OnRep_LED State`
  (bind _cooldown_timer (`self.cooldown timer`))
  (`|ExecutionSequence`
    (:`then_0`
      (switch `string` (`self.LED State`)
        (:`Default`
          (if (`KismetSystemLibrary.K2_IsValidTimerHandle` _cooldown_timer)
            (`KismetSystemLibrary.K2_ClearAndInvalidateTimerHandle` _cooldown_timer)))
        (:`cooldown`
          (bind _returnvalue (`KismetSystemLibrary.K2_SetTimer` null "cooldown ended" (`self.cooldown`)))
          (set `self.cooldown timer` _returnvalue))))
    (:`then_1`
      (`self.update outline`))))

(fn `OnRep_name`)

(fn `OnRep_symbol`)

(fn `OnRep_targetSkewOffset`)

(fn `Set Key Mesh`
  (params (type :type Name) (color :type "LinearColor Structure") (emission :type "LinearColor Structure") (`custom color` :type Boolean) (`static mesh ` :type "StaticMesh Soft Object Reference") (KeycapSpawnData :type "/Game/data/FKeycapSpawnData Structure"))
  (bind _staticmesh (break `/Game/data/FKeycapSpawnData` KeycapSpawnData))
  (bind _staticmesh_2 (`self.StaticMesh`))
  (bind _labeltarget (`self.LabelTarget`))
  ;[1 1 1] add new mesh
  (`StaticMeshComponent.SetStaticMesh` (`self.StaticMesh`) _staticmesh)
  (`StaticMeshComponent.SetStaticMesh` (`self.StaticMeshForOutline`) _staticmesh)
  ;[1 1 1] set label rotations
  (switch `name` (`self.KeyCapType`)
    (:`Default`
      (`SceneComponent.K2_SetRelativeRotation` _labeltarget (struct :`Yaw` 180.0) false false))
    (:`realboyv1`
      (`SceneComponent.K2_SetRelativeRotation` _labeltarget (struct :`Pitch` 90.0 :`Yaw` 180.0) false false)))
  ;[1 1 1] set mesh rotations
  (switch `name` (`self.KeyCapType`)
    (:`Default`
      (`SceneComponent.K2_SetRelativeRotation` :`self` _staticmesh_2))
    (:`trickyv1`
      (`SceneComponent.K2_SetRelativeRotation` _staticmesh_2 (`KismetMathLibrary.MakeRotator` 0.0 0.0 (`KismetMathLibrary.Conv_IntToDouble` (* (`self.index`) 15))) false false))))

(fn `setKeyActive`
  (params (active :type Boolean) (shiftIsActive :type Boolean))
  ;[1 1 1] double tap logic
  (if (`KismetStringLibrary.NotEqual_StrStr` (`self.LED State`) "cooldown")
    (if active
      (bind _asbp_game_state (cast `/Game/Core/BP_GameState` (`GameplayStatics.GetGameState`)))
      (if (and (< (- (`KismetSystemLibrary.GetGameTimeInSeconds`) (`self.Last Pressed`)) 0.2) (`/Game/Core/BP_GameState.mod-active-double tap` _asbp_game_state))
        (set `self.key speed` 0.6)
        (set `self.DblTap Is Active` true)
        (set `self.LED State` "fast active")
        (else
          (set `self.key speed` 0.17)
          (set `self.DblTap Is Active` false)
          (set `self.LED State` "active")))
      (if (`KismetStringLibrary.NotEqual_StrStr` (`self.LED State`) "cooldown")
        (set `self.Last Pressed` (`KismetSystemLibrary.GetGameTimeInSeconds`)))
      (else
        (set `self.key speed` 0.17)
        (if (> (`self.cooldown`) 0.0)
          (set `self.LED State` "cooldown")
          (else
            (set `self.LED State` "inactive")))))
    (bind _output_get (set `self.isActive` active))
    (if _output_get
      (bind _output_get_2 (set `self.Shift Is Active` shiftIsActive))
      (if (and _output_get _output_get_2)
        (set `self.LED State` "shift active"))
      (if _output_get_2
        (set `self.Z_Active_Value` (`self.specialTargetZ`))
        (else
          (set `self.Z_Active_Value` (`self.normalTargetZ`))))
      (elif (`KismetStringLibrary.NotEqual_StrStr` (`self.LED State`) "cooldown")
        (set `self.Last Released` (`KismetSystemLibrary.GetGameTimeInSeconds`))))))

(fn `setOrganicKeyMesh`
  (params (staticMeshComponent :type "StaticMesh Object Reference"))
  (bind _staticmesh (`self.StaticMesh`))
  (bind (_min _max) (`StaticMeshComponent.GetLocalBounds` _staticmesh))
  (bind _returnvalue (/ (+ _min _max) 2.0))
  (bind _x (.x _returnvalue))
  (bind _z (.z _returnvalue))
  (bind _returnvalue_2 (+ (.y _returnvalue) 65.0))
  (set `self.organic` true)
  (`StaticMeshComponent.SetStaticMesh` (`self.StaticMesh`) staticMeshComponent)
  (set `self.base organic mesh offset` _returnvalue)
  (`self.K2_SetActorLocation` self (`KismetMathLibrary.MakeVector` _x _returnvalue_2 _z) false false)
  (bind _output_get (set `self.originLocation` (`KismetMathLibrary.MakeVector` _x _returnvalue_2 _z)))
  (set `self.targetPosition` _output_get)
  (`SceneComponent.K2_SetRelativeLocation` _staticmesh (* _returnvalue -1) false false)
  (`StaticMeshComponent.SetStaticMesh` (`self.StaticMeshForOutline`) staticMeshComponent))

(fn `Toggle Between The Primary And Secondary Key Mesh`
  (switch `name` (`self.activeCapPrimaryOrSecondary`)
    (:`primary`
      (set `self.activeCapPrimaryOrSecondary` "secondary"))
    (:`secondary`
      (set `self.activeCapPrimaryOrSecondary` "primary")))
  (bind _active_mod (message `/Game/Core/BPI_GameState.Get Active Mod` (`GameplayStatics.GetGameState`)))
  (switch `name` (`self.activeCapPrimaryOrSecondary`)
    (:`primary`
      (switch `int` (`self.teamIndex`)
        (:`0`
          (bind _returnvalue (`VaRestJsonObject.GetObjectField` _active_mod "keycaps"))
          (`self.Set Key Mesh` (`KismetStringLibrary.Conv_StringToName` (`VaRestJsonObject.GetStringField` _returnvalue "primary left"))))
        (:`1`
          (`self.Set Key Mesh` (`KismetStringLibrary.Conv_StringToName` (`VaRestJsonObject.GetStringField` _returnvalue "primary right"))))))
    (:`secondary`
      (switch `int` (`self.teamIndex`)
        (:`0`
          (`self.Set Key Mesh` (`KismetStringLibrary.Conv_StringToName` (`VaRestJsonObject.GetStringField` _returnvalue "secondary left"))))
        (:`1`
          (`self.Set Key Mesh` (`KismetStringLibrary.Conv_StringToName` (`VaRestJsonObject.GetStringField` _returnvalue "secondary right"))))))))

(fn `UserConstructionScript`
  (bind (_returnvalue_x _returnvalue_y _returnvalue_z) (`KismetMathLibrary.BreakVector` (`self.K2_GetActorLocation`)))
  (bind _returnvalue (`GameplayStatics.GetActorOfClass` "/Game/Core/BP_Camera.BP_Camera_C"))
  (set `self.main camera` _returnvalue)
  (set `self.inactiveZ` _returnvalue_z))