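; Game state that holds team scores and the active play, court and ball modes, with getters for score, mode and player count.
; Mode switches swap blocking streamed sublevels named after each mode and restyle keys on BP_Keyboard.
; Court switches to or from chess also change the ball mode, and SetCam messages the "main"-tagged camera.
; Match-end, winner widget and key layout logic is disconnected, and LobbyState's OnRep only prints debug text.
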(event `self.ReceiveBeginPlay`
  (bind _returnvalue (`GameplayStatics.GetActorOfClass` "/Game/Core/BP_Keyboard.BP_Keyboard_C"))
  (set `self.keyboard` _returnvalue))

(event `self.setPlayMode`
  (params (val :type String))
  (`GameplayStatics.UnloadStreamLevel` (`KismetStringLibrary.Conv_StringToName` (`self.PlayMode`)) true)
  (bind _output_get (set `self.PlayMode` val))
  (message `/Game/Core/BPI_Keyboard.setPlayModeKeyStyles` (`self.keyboard`) _output_get)
  (`GameplayStatics.LoadStreamLevel` (`KismetStringLibrary.Conv_StringToName` (`self.PlayMode`)) true true))

(event `self.setCam`
  (params (val :type String))
  (bind _outactors (`GameplayStatics.GetAllActorsOfClassWithTag` "/Script/Engine.CameraActor" "main"))
  (message `/Game/Core/BPI_GameState.setCam` (`|GetArrayItem` _outactors) val))

(event `self.switchCourt`
  (params (val :type String))
  (bind _activecourtmode (`self.ActiveCourtMode`))
  (bind _activecourtmode_2 (`self.ActiveCourtMode`))
  (`GameplayStatics.UnloadStreamLevel` (`KismetStringLibrary.Conv_StringToName` _activecourtmode) true)
  (if (`KismetStringLibrary.EqualEqual_StrStr` _activecourtmode "chess")
    (`self.switchBall` self "keyball")
    (else
      (bind _output_get (set `self.ActiveCourtMode` val))
      (message `/Game/Core/BPI_Keyboard.setPlayModeKeyStyles` (`self.keyboard`) _output_get)
      (`GameplayStatics.LoadStreamLevel` (`KismetStringLibrary.Conv_StringToName` _activecourtmode_2) true true)
      (if (`KismetStringLibrary.EqualEqual_StrStr` _activecourtmode_2 "chess")
        (`self.switchBall` self "none")))))

(event `self.setRandomModeActive`
  (params (NewParam :type Boolean))
  (set `self.randomModeActive` NewParam))

(event `self.switchBall`
  (params (val :type String))
  (`GameplayStatics.UnloadStreamLevel` (`KismetStringLibrary.Conv_StringToName` (`self.ActiveBallMode`)) true)
  (bind _output_get (set `self.ActiveBallMode` val))
  (message `/Game/Core/BPI_Keyboard.setPlayModeKeyStyles` (`self.keyboard`) _output_get)
  (`GameplayStatics.LoadStreamLevel` (`KismetStringLibrary.Conv_StringToName` (`self.ActiveBallMode`)) true true))

(event `self.set score`
  (params (`which team ` :type String) (`new score` :type Integer))
  (switch `string` `which team `
    (:`team1`
      (set `self.team1_score` `new score`))
    (:`team2`
      (set `self.team2_score` `new score`))))

(fn `Get Active Mod`
  (returns (`active mod` :type "VaRestJsonObject Object Reference"))
  (return (`self.active game mod`)))

(fn `get player count`
  (returns (current :type Integer) (target :type Integer))
  (bind _numconnections (`AdvancedSessionsLibrary.GetSessionSettings`)
    (:`OnSuccess`
      (return (`KismetArrayLibrary.Array_Length` (`self.PlayerArray`)) _numconnections))))

(fn `get score`
  (returns (team1 :type Integer) (team2 :type Integer))
  (return (`self.team1_score`) (`self.team2_score`)))

(fn `getPlayMode`
  (returns (PlayMode :type String))
  (return (`self.PlayMode`)))

(fn `OnRep_LobbyState`
  (`KismetSystemLibrary.PrintString` (`KismetStringLibrary.Concat_StrStr` "LOBBY STATE CHANGED :O 1  " (`VaRestJsonObject.GetStringField` (`self.Lobby Settings2`) "primary left")) true true (struct :`G` 0.66 :`B` 1.0 :`A` 1.0) 20.0))

(fn `OnRep_winner`)

(fn `UserConstructionScript`
  (bind _returnvalue (`GameplayStatics.GetActorOfClass` "/Game/Core/BP_Keyboard.BP_Keyboard_C"))
  (set `self.keyboard` _returnvalue))