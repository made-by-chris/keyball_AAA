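; BP_ShelfGenerator builds a shelf display of keyboards from the KeyboardDataAsset data table.
; Its construction script adds a BP_DisplayKeyboard child actor per row, slightly rotated and placed on a Y/Z grid set by column count and spacing.
; A cumulative per-index offset also shifts each one along Y.
; Each actor's Setup receives the row's name, type, status, struct and one-based ID, alongside a debug print of the type.
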(fn `UserConstructionScript`
  (locals (NewLocalVar_0 :type String :default "spawning the ") (NewLocalVar_1 :type String :default "display keyboard"))
  (bind _keyboarddataasset (`self.KeyboardDataAsset`))
  (bind _outrownames (`DataTableFunctionLibrary.GetDataTableRowNames` _keyboarddataasset))
  (for (_array_element _array_index) _outrownames
    (bind _returnvalue (`|GetDataTableRow` _keyboarddataasset _array_element)
      (:`then`
        (bind _output_get (set `self.keyboardStruct` _returnvalue))
        (`KismetSystemLibrary.PrintString` (`KismetStringLibrary.Concat_StrStr` "SHELFFFF     " (`|GetEnumeratorNameAsString` (`.keyboardType_14_B3CA1148DF4166415F4055AF802E1E64` (break `/Game/data/KeyboardDataStruct` _output_get)))))
        (bind _returnvalue_2 (`AddComponent|NODE_AddChildActorComponent-0` :`RelativeTransform` (`KismetMathLibrary.MakeTransform` (`KismetMathLibrary.MakeVector` 0.0 (+ (* (`KismetMathLibrary.FTrunc` (mod (`KismetMathLibrary.Conv_IntToDouble` _array_index) (`KismetMathLibrary.Conv_IntToDouble` (`self.nColumns`)))) (`self.spacingX`)) (* _array_index -20.0)) (* (/ _array_index (`self.nColumns`)) (`self.spacingY`))) (struct :`Pitch` 10.0))))
        (`ChildActorComponent.SetChildActorClass` _returnvalue_2 "/Game/Core/BP_DisplayKeyboard.BP_DisplayKeyboard_C")
        (bind _asbp_display_keyboard (cast `/Game/Core/BP_DisplayKeyboard` (`ChildActorComponent.ChildActor` _returnvalue_2)))
        (`/Game/Core/BP_DisplayKeyboard.setup` _asbp_display_keyboard (break `/Game/data/KeyboardDataStruct` _output_get) (`.keyboardType_14_B3CA1148DF4166415F4055AF802E1E64` (break `/Game/data/KeyboardDataStruct` _output_get)) (`.status_8_C196D578EF48F104CDA97082A38E3BF4` (break `/Game/data/KeyboardDataStruct` _output_get)) _returnvalue (+ _array_index 1))))))